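; Combat director that coordinates enemy AI around the player by sorting registered controllers into idle, outer ring and inner ring groups.
; AIUpdate returns each controller's next state, promoting idle AIs within view distance to distancing, then to targeting as inner slots open.
; An outer AI inside the inner radius takes a slot, displacing the farthest member if full.
; A looping timer orders a random inner AI to attack; Tick draws debug ring spheres.
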(event `self.ReceiveBeginPlay`
  ;[1 1 1] The player is 99% of the time going to be the combat directors main target so we set it here
  (set `self.MainTarget` (`GameplayStatics.GetPlayerCharacter` 0))
  (`KismetSystemLibrary.K2_SetTimerDelegate` (delegate `BeginAttack`) (`self.AttackInterval`) true))

(event `self.ReceiveTick`
  (params (DeltaSeconds :type "Float (single-precision)"))
  (`KismetSystemLibrary.DrawDebugSphere` (`self.K2_GetActorLocation` (`self.MainTarget`)) (`self.InnerRingRadius`) 12 (struct :`R` 1.0 :`A` 1.0) 0.0 1.0)
  (`KismetSystemLibrary.DrawDebugSphere` (`self.K2_GetActorLocation` (`self.MainTarget`)) (`self.OutsideRingRadius`) 12 (struct :`R` 1.0 :`A` 1.0) 0.0 1.0))

(event `BeginAttack`
  (bind _innerringais (`self.InnerRingAIs`))
  (if (`KismetArrayLibrary.Array_IsNotEmpty` _innerringais)
    (`/Game/_Main/Blueprints/AI/BP_EnemyAIController.Update State` (`KismetArrayLibrary.Array_Random` _innerringais) "NewEnumerator2")))

(fn `AIUpdate`
  (params (`Controller Instance` :type "AIController Object Reference") (`Current State` :type "/Game/_Main/Blueprints/AI/E_AIStates Enum" :default "NewEnumerator0") (`Distance To Target` :type "Float (double-precision)"))
  (returns (`New State` :type "/Game/_Main/Blueprints/AI/E_AIStates Enum"))
  (bind _asbp_enemy_aicontroller (cast `/Game/_Main/Blueprints/AI/BP_EnemyAIController` `Controller Instance`))
  (switch `/Game/_Main/Blueprints/AI/E_AIStates` `Current State`
    (:`NewEnumerator0`
      (bind _new_state (`self.AIUpdateIDLE` _asbp_enemy_aicontroller `Distance To Target`))
      (return _new_state))
    (:`NewEnumerator1`
      (bind _newstate (`self.AIUpdateDISTANCING` _asbp_enemy_aicontroller `Distance To Target`))
      (return _newstate))
    (:`NewEnumerator4`
      _)
    (:`NewEnumerator2`
      _)
    (:`NewEnumerator3`
      _))
  (return `Current State`))

(fn `AIUpdateDISTANCING`
  (params (Controller :type "/Game/_Main/Blueprints/AI/BP_EnemyAIController Object Reference") (DistanceToTarget :type "Float (double-precision)"))
  (returns (NewState :type "/Game/_Main/Blueprints/AI/E_AIStates Enum"))
  (locals (Local_FurthestIndex :type Integer) (Local_FurthestDistance :type "Float (double-precision)"))
  (if (< (`KismetArrayLibrary.Array_Length` (`self.InnerRingAIs`)) (`self.TargetInnerRingEnemiesCount`))
    (`KismetArrayLibrary.Array_RemoveItem` (`self.OuterRingAIs`) Controller)
    (`KismetArrayLibrary.Array_Add` (`self.InnerRingAIs`) Controller)
    (return "NewEnumerator4")
    (else
      ;[1 1 1] If the outer ring AI is now close (because of player moving quickly) we need to add it to the inner and remove a far enemy (if at inner limit)
      (if (<= DistanceToTarget (`self.InnerRingRadius`))
        (`self.InsertToInnerAndRegroup` Controller)
        (return "NewEnumerator4")
        (else
          (return "NewEnumerator1"))))))

(fn `AIUpdateIDLE`
  (params (Controller :type "/Game/_Main/Blueprints/AI/BP_EnemyAIController Object Reference") (`Distance To Target` :type "Float (double-precision)"))
  (returns (`New State` :type "/Game/_Main/Blueprints/AI/E_AIStates Enum"))
  (if (<= `Distance To Target` (`/Game/_Main/Blueprints/AI/BP_EnemyAIController.View Distance` Controller))
    (`KismetArrayLibrary.Array_RemoveItem` (`self.IdleAIs`) Controller)
    (`KismetArrayLibrary.Array_Add` (`self.OuterRingAIs`) Controller)
    (return "NewEnumerator1")
    (else
      (return "NewEnumerator0"))))

(fn `InsertToInnerAndRegroup`
  (params (ControllerToInsert :type "/Game/_Main/Blueprints/AI/BP_EnemyAIController Object Reference"))
  (locals (Local_FurthestIndex :type Integer) (Local_FurthestDistance :type "Float (double-precision)"))
  (bind _output (`|GetArrayItem` (`self.InnerRingAIs`) (`local.Local_FurthestIndex`)))
  ;[1 1 1] See if we have room in the inner ring to just insert the AI without regrouping
  (if (not (< (`KismetArrayLibrary.Array_Length` (`self.InnerRingAIs`)) (`self.TargetInnerRingEnemiesCount`)))
    ;[1 1 1] Find the furthest AI in the inner group to remove
    (for (_array_element _array_index) (`self.InnerRingAIs`)
      (bind _returnvalue (`KismetMathLibrary.Abs` (`KismetMathLibrary.Vector_Distance` (`self.K2_GetActorLocation` (`self.MainTarget`)) (`self.K2_GetActorLocation` _array_element))))
      (if (> _returnvalue (`local.Local_FurthestDistance`))
        (set `local.Local_FurthestDistance` _returnvalue)
        (set `local.Local_FurthestIndex` _array_index)))
    ;[1 1 1] Remove the chosen AI from the inner group
    (`/Game/_Main/Blueprints/AI/BP_EnemyAIController.Update State` _output "NewEnumerator1")
    (`KismetArrayLibrary.Array_Add` (`self.OuterRingAIs`) _output)
    (`KismetArrayLibrary.Array_RemoveItem` (`self.InnerRingAIs`) _output))
  (`KismetArrayLibrary.Array_Add` (`self.InnerRingAIs`) ControllerToInsert)
  (`KismetArrayLibrary.Array_RemoveItem` (`self.OuterRingAIs`) ControllerToInsert))

(fn `RegisterAI`
  (params (AI :type "/Game/_Main/Blueprints/AI/BP_EnemyAIController Object Reference"))
  (`KismetArrayLibrary.Array_Add` (`self.IdleAIs`) AI)
  (`BlackboardComponent.SetValueAsObject` (`AIBlueprintHelperLibrary.GetBlackboard` AI) "CombatDirector" self)
  (`/Game/_Main/Blueprints/AI/BP_EnemyAIController.Update State` AI "NewEnumerator0"))

(fn `UnRegisterAI`
  (params (Controller :type "/Game/_Main/Blueprints/AI/BP_EnemyAIController Object Reference"))
  (bind _returnvalue (`KismetArrayLibrary.Array_RemoveItem` (`self.InnerRingAIs`) Controller))
  (if (not _returnvalue)
    (`KismetArrayLibrary.Array_RemoveItem` (`self.OuterRingAIs`) Controller)))

(fn `UserConstructionScript`)