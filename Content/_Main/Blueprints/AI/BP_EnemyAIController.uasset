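; Enemy AI controller that runs the BT_EnemyAI behavior tree and registers itself with the BP_AICombatDirector found in the level.
; On BeginPlay it seeds the blackboard with view distance, home radius and its own starting location as the home position.
; UpdateState stores the current AI state, mirrors it to the blackboard and prints it.
; Small helper functions wrap blackboard writes for float, vector and object keys.
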(event `self.ReceiveBeginPlay`
  (`self.RunBehaviorTree` "/Game/_Main/Blueprints/AI/BT_EnemyAI.BT_EnemyAI")
  (`self.Set BlackboardValues`)
  (bind _returnvalue (`GameplayStatics.GetActorOfClass` "/Game/_Main/Blueprints/AI/BP_AICombatDirector.BP_AICombatDirector_C"))
  (`/Game/_Main/Blueprints/AI/BP_AICombatDirector.RegisterAI` _returnvalue self))

(fn `Set Black Board Float`
  (params (`Key Name` :type Name) (Value :type "Float (double-precision)"))
  (`BlackboardComponent.SetValueAsFloat` (`AIBlueprintHelperLibrary.GetBlackboard` null) `Key Name` Value))

(fn `Set Black Board Object`
  (params (`Key Name` :type Name) (Value :type "Object Object Reference (by ref)"))
  (`BlackboardComponent.SetValueAsObject` (`AIBlueprintHelperLibrary.GetBlackboard` null) `Key Name` Value))

(fn `Set Black Board Vector`
  (params (`Key Name` :type Name) (Value :type "Vector Structure"))
  (`BlackboardComponent.SetValueAsVector` (`AIBlueprintHelperLibrary.GetBlackboard` null) `Key Name` Value))

(fn `Set BlackboardValues`
  (`self.Set Black Board Float` "ViewDistance" (`self.View Distance`))
  (`self.Set Black Board Float` "HomeRadius" (`self.Home Radius`))
  (`self.Set Black Board Vector` "HomePosition" (`self.K2_GetActorLocation`)))

(fn `Update State`
  (params (NewState :type "/Game/_Main/Blueprints/AI/E_AIStates Enum" :default "NewEnumerator0"))
  (bind _output_get (set `self.CurrentAIState` NewState))
  (`BlackboardComponent.SetValueAsEnum` (`AIBlueprintHelperLibrary.GetBlackboard` null) "AIState" _output_get)
  (`KismetSystemLibrary.PrintString` (`|GetEnumeratorNameAsString` _output_get)))

(fn `UserConstructionScript`)