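; Behavior tree service that sets an AI pawn's target position on a ring around the combat director's main target.
; On tick, the DISTANCING state uses the outside ring radius and TARGETING the inner one.
; It projects the pawn's 2D direction from the target onto that ring, then writes a nearby navigable point to the blackboard.
; An uncalled, unfinished AdjustPosition helper tests line of sight and rotates blocked positions.
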(event `self.ReceiveTickAI`
  (params (OwnerController :type "AIController Object Reference") (ControlledPawn :type "Pawn Object Reference") (DeltaSeconds :type "Float (single-precision)"))
  (bind _asbp_aicombat_director (cast `/Game/_Main/Blueprints/AI/BP_AICombatDirector` (`BTFunctionLibrary.GetBlackboardValueAsObject` (`self.IN OBJ - CombatDirector`))))
  (switch `/Game/_Main/Blueprints/AI/E_AIStates` (cast `/Game/_Main/Blueprints/AI/E_AIStates` (`BTFunctionLibrary.GetBlackboardValueAsEnum` (`self.IN STATE - AI State`)))
    (:`NewEnumerator1`
      (bind _maintarget (`/Game/_Main/Blueprints/AI/BP_AICombatDirector.MainTarget` _asbp_aicombat_director))
      (bind _position (`self.CalculateNearestRingPosition` _maintarget ControlledPawn (`/Game/_Main/Blueprints/AI/BP_AICombatDirector.OutsideRingRadius` _asbp_aicombat_director)))
      (bind _randomlocation (`NavigationSystemV1.K2_GetRandomLocationInNavigableRadius` _position 5.0 null null))
      (`BTFunctionLibrary.SetBlackboardValueAsVector` (`self.OUT VEC - Target Position`) _randomlocation))
    (:`NewEnumerator4`
      (bind _position_2 (`self.CalculateNearestRingPosition` _maintarget ControlledPawn (`/Game/_Main/Blueprints/AI/BP_AICombatDirector.InnerRingRadius` _asbp_aicombat_director)))
      (bind _randomlocation_2 (`NavigationSystemV1.K2_GetRandomLocationInNavigableRadius` _position_2 5.0 null null))
      (`BTFunctionLibrary.SetBlackboardValueAsVector` (`self.OUT VEC - Target Position`) _randomlocation_2))))

(fn `AdjustPosition`
  (params (CalculatedPosition :type "Vector Structure") (RingOriginActor :type "Actor Object Reference") (MovingActor :type "Actor Object Reference"))
  (returns (NewPosition :type "Vector Structure"))
  (bind _ascontroller (cast `Controller` RingOriginActor)
    (:`then`
      (if (`Controller.LineOfSightTo` _ascontroller MovingActor (0.0 0.0 0.0) false)
        (return CalculatedPosition)
        (else
          (`KismetSystemLibrary.PrintString` "Hello")
          (if (> (`KismetMathLibrary.Dot_VectorVector` (- (`Actor.K2_GetActorLocation` MovingActor) (`Actor.K2_GetActorLocation` RingOriginActor)) (`Actor.GetActorForwardVector` RingOriginActor)) 0.0)
            (return (`KismetMathLibrary.RotateAngleAxis` CalculatedPosition 5.0 (0.0 0.0 1.0)))
            (else
              (return (`KismetMathLibrary.RotateAngleAxis` CalculatedPosition 5.0 (0.0 0.0 1.0))))))))
    (:`CastFailed`
      (`KismetSystemLibrary.PrintString` "AAAAAAAAAAAAA"))))

(fn `CalculateNearestRingPosition`
  (params (RingCenterPawn :type "Pawn Object Reference") (MovingPawn :type "Pawn Object Reference") (RingRadius :type "Float (double-precision)"))
  (returns (Position :type "Vector Structure"))
  (bind _returnvalue (`Actor.K2_GetActorLocation` RingCenterPawn))
  (return (+ (`KismetMathLibrary.MakeVector` (* (.x (`KismetMathLibrary.Vector_Normal2D` (- (`Actor.K2_GetActorLocation` MovingPawn) _returnvalue))) RingRadius) (* (.y (`KismetMathLibrary.Vector_Normal2D` (- (`Actor.K2_GetActorLocation` MovingPawn) _returnvalue))) RingRadius) (`.Z` (`KismetMathLibrary.BreakVector3f` _returnvalue))) _returnvalue)))