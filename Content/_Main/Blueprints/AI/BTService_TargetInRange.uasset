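; Behavior tree service that notifies the combat director when an AI pawn is within range of the director's main target.
; Each tick it reads the BP_AICombatDirector from the blackboard and compares pawn-to-target distance against the blackboard view distance.
; Despite the "CanSee" name, the check is distance only, with no line of sight.
; When in range, it passes the BP_EnemyAIController to AIInRangeOfTarget; leaving range triggers no call.
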(event `self.ReceiveTickAI`
  (params (OwnerController :type "AIController Object Reference") (ControlledPawn :type "Pawn Object Reference") (DeltaSeconds :type "Float (single-precision)"))
  (bind _asaicombat_director (cast `/Game/_Main/Blueprints/AI/BP_AICombatDirector` (`BTFunctionLibrary.GetBlackboardValueAsObject` (`self.IN OBJ - Combat Director`))))
  (bind _can_see (`self.Can See Combat Director Target` ControlledPawn _asaicombat_director))
  (if _can_see
    (bind _asbp_enemy_aicontroller (cast `/Game/_Main/Blueprints/AI/BP_EnemyAIController` OwnerController))
    (`/Game/_Main/Blueprints/AI/BP_AICombatDirector.AIInRangeOfTarget` _asaicombat_director _asbp_enemy_aicontroller)))

(fn `Can See Combat Director Target`
  (params (`AI Pawn` :type "Pawn Object Reference") (CombatDirector :type "/Game/_Main/Blueprints/AI/BP_AICombatDirector Object Reference"))
  (returns (`Can See` :type Boolean))
  (return (<= (`KismetMathLibrary.Vector_Distance` (`Actor.K2_GetActorLocation` `AI Pawn`) (`Actor.K2_GetActorLocation` (`/Game/_Main/Blueprints/AI/BP_AICombatDirector.MainTarget` CombatDirector))) (`BTFunctionLibrary.GetBlackboardValueAsFloat` (`self.IN FLOAT - View Distance`)))))