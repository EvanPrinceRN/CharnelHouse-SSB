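; Behavior tree service that syncs an AI with the combat director stored in its blackboard.
; Each tick it passes the controller, current state and pawn's distance to the director's main target into the director's AIUpdate.
; The returned state is written back to the same blackboard key.
; Focus is set to empty for IDLE and to the main target for DISTANCING; other states leave it untouched.
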(event `self.ReceiveTickAI`
  (params (OwnerController :type "AIController Object Reference") (ControlledPawn :type "Pawn Object Reference") (DeltaSeconds :type "Float (single-precision)"))
  (bind _asbp_aicombat_director (cast `/Game/_Main/Blueprints/AI/BP_AICombatDirector` (`BTFunctionLibrary.GetBlackboardValueAsObject` (`self.IN OBJ - Combat Director`))))
  (bind _distance (`self.GetDistanceToTarget` (`/Game/_Main/Blueprints/AI/BP_AICombatDirector.MainTarget` _asbp_aicombat_director) ControlledPawn))
  (bind _new_state (`/Game/_Main/Blueprints/AI/BP_AICombatDirector.AIUpdate` _asbp_aicombat_director OwnerController (cast `/Game/_Main/Blueprints/AI/E_AIStates` (`BTFunctionLibrary.GetBlackboardValueAsEnum` (`self.IN OUT STATE - Current State`))) _distance))
  (`BTFunctionLibrary.SetBlackboardValueAsEnum` (`self.IN OUT STATE - Current State`) _new_state)
  (switch `/Game/_Main/Blueprints/AI/E_AIStates` _new_state
    (:`NewEnumerator0`
      (`AIController.K2_SetFocus` OwnerController null))
    (:`NewEnumerator1`
      (`AIController.K2_SetFocus` OwnerController (`/Game/_Main/Blueprints/AI/BP_AICombatDirector.MainTarget` _asbp_aicombat_director)))))

(fn `GetDistanceToTarget`
  (params (Target :type "Character Object Reference") (`Controlled Pawn` :type "Pawn Object Reference"))
  (returns (Distance :type "Float (double-precision)"))
  (return (`KismetMathLibrary.Abs` (`KismetMathLibrary.Vector_Distance` (`Actor.K2_GetActorLocation` Target) (`Actor.K2_GetActorLocation` `Controlled Pawn`)))))