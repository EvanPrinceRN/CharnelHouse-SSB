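; Anim notify state that deals melee weapon damage while active on a BP_CharacterBase animation.
; Each tick it loops over the owner's Weapons, sphere-tracing between two mesh sockets on the Camera channel with debug drawing, though returns in the loop body exit after the first trace.
; Hits on characters of a different Type receive that weapon's damage and set AnimationHitLock, limiting damage to one hit until NotifyEnd clears it.
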(fn `Get Character Base`
  (params (MeshComponent :type "MeshComponent Object Reference"))
  (returns (CharacterBase :type "/Game/_Main/Blueprints/BP_CharacterBase Object Reference"))
  (bind _asbp_character_base (cast `/Game/_Main/Blueprints/BP_CharacterBase` (`ActorComponent.GetOwner` MeshComponent))
    (:`then`
      (return _asbp_character_base))
    (:`CastFailed`
      (`KismetSystemLibrary.PrintString` null "Invalid character for anim notify"))))

(fn `Received_NotifyEnd`
  (params (MeshComp :type "SkeletalMeshComponent Object Reference") (Animation :type "AnimSequenceBase Object Reference") (EventReference :type "AnimNotifyEventReference Structure (by ref)"))
  (returns (ReturnValue :type Boolean))
  ;[1 1 1] Reset the hit lock
  (bind _characterbase (`self.Get Character Base` MeshComp))
  (set `/Game/_Main/Blueprints/BP_CharacterBase.AnimationHitLock` false _characterbase)
  (return false))

(fn `Received_NotifyTick`
  (params (MeshComp :type "SkeletalMeshComponent Object Reference") (Animation :type "AnimSequenceBase Object Reference") (FrameDeltaTime :type "Float (single-precision)") (EventReference :type "AnimNotifyEventReference Structure (by ref)"))
  (returns (ReturnValue :type Boolean))
  (locals (LOCAL_CharacterBase :type "/Game/_Main/Blueprints/BP_CharacterBase Object Reference") (LOCAL_MeshComp :type "MeshComponent Object Reference") (LOCAL_Hit :type "HitResult Structure") (LOCAL_ThisWeapon :type "/Game/_Main/Blueprints/WeaponDetails Structure"))
  (bind _local_meshcomp (`local.LOCAL_MeshComp`))
  (bind _local_characterbase (`local.LOCAL_CharacterBase`))
  (bind _output_get (set `local.LOCAL_MeshComp` MeshComp))
  (bind _characterbase (`self.Get Character Base` _output_get))
  (bind _output_get_2 (set `local.LOCAL_CharacterBase` _characterbase))
  ;[1 1 1] Check if we have already hit during this animation
  (if (`/Game/_Main/Blueprints/BP_CharacterBase.AnimationHitLock` _output_get_2)
    (return false)
    (else
      ;[1 1 1] Check each weapon for a hit
      (for _array_element (`/Game/_Main/Blueprints/BP_CharacterBase.Weapons` (`local.LOCAL_CharacterBase`))
        (bind _output_get_3 (set `local.LOCAL_ThisWeapon` _array_element))
        (bind (_weaponsocketname1 _weakponsocketname2 _collisiondetectionradius) (break `/Game/_Main/Blueprints/WeaponDetails` _output_get_3))
        (bind (_outhit _returnvalue) (`KismetSystemLibrary.SphereTraceSingle` :`WorldContextObject` _local_meshcomp :`Start` (`SceneComponent.GetSocketLocation` _local_meshcomp _weaponsocketname1) :`End` (`SceneComponent.GetSocketLocation` _local_meshcomp _weakponsocketname2) :`Radius` _collisiondetectionradius :`TraceChannel` "TraceTypeQuery2" :`DrawDebugType` "ForDuration"))
        (set `local.LOCAL_Hit` _outhit)
        ;[1 1 1] Have we hit?
        (if _returnvalue
          ;[1 1 1] Is the hit character type different to the attacker type? (This is to prevent an enemy hitting another enemy when close)
          (bind _asbp_character_base (cast `/Game/_Main/Blueprints/BP_CharacterBase` (`.HitActor` (`GameplayStatics.BreakHitResult` (`local.LOCAL_Hit`)))))
          (if (`|EnumInequality` (`/Game/_Main/Blueprints/BP_CharacterBase.Type` _asbp_character_base) (`/Game/_Main/Blueprints/BP_CharacterBase.Type` (`local.LOCAL_CharacterBase`)))
            ;[1 1 1] Apply the damage
            (set `/Game/_Main/Blueprints/BP_CharacterBase.AnimationHitLock` true _local_characterbase)
            (`GameplayStatics.ApplyDamage` (`.HitActor` (`GameplayStatics.BreakHitResult` (`local.LOCAL_Hit`))) (`.Damage_9_5CD86A22411910317081A1B6FC474CE3` (break `/Game/_Main/Blueprints/WeaponDetails` (`local.LOCAL_ThisWeapon`))) null _local_characterbase)
            (return false)
            (else
              (return false)))
          (else
            (return false)))))))