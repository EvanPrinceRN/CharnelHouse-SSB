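; Anim notify state for Enemy1 attacks that deals damage to whatever its hands touch during the notify window.
; Each tick it runs zero-length sphere traces on the Camera channel at the right, then left, middle-finger sockets.
; A hit on either hand feeds a shared ApplyDamage call with a fixed amount.
; No hit actors are tracked, so damage can repeat every tick while overlap lasts.
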(fn `Received_NotifyTick`
  (params (MeshComp :type "SkeletalMeshComponent Object Reference") (Animation :type "AnimSequenceBase Object Reference") (FrameDeltaTime :type "Float (single-precision)") (EventReference :type "AnimNotifyEventReference Structure (by ref)"))
  (returns (ReturnValue :type Boolean))
  (locals (Local_Radius :type "Float (double-precision)" :default 10.0) (Local_DrawDebug :type "EDrawDebugTrace Enum" :default "ForDuration") (Local_Hit :type "HitResult Structure"))
  (bind _returnvalue (`SceneComponent.GetSocketLocation` MeshComp "middle_01_r"))
  (bind _returnvalue_2 (`SceneComponent.GetSocketLocation` MeshComp "middle_01_l"))
  (`|ExecutionSequence`
    (:`then_0`
      (bind (_outhit _returnvalue_3) (`KismetSystemLibrary.SphereTraceSingle` :`WorldContextObject` MeshComp :`Start` _returnvalue :`End` _returnvalue :`Radius` (`local.Local_Radius`) :`TraceChannel` "TraceTypeQuery2" :`DrawDebugType` (`local.Local_DrawDebug`)))
      (if _returnvalue_3
        (set `local.Local_Hit` _outhit)
        (`GameplayStatics.ApplyDamage` (`.HitActor` (`GameplayStatics.BreakHitResult` (`local.Local_Hit`))) 10.0 :!label _label)
        (return false)))
    (:`then_1`
      (bind (_outhit_2 _returnvalue_4) (`KismetSystemLibrary.SphereTraceSingle` :`WorldContextObject` MeshComp :`Start` _returnvalue_2 :`End` _returnvalue_2 :`Radius` (`local.Local_Radius`) :`TraceChannel` "TraceTypeQuery2" :`DrawDebugType` (`local.Local_DrawDebug`)))
      (if _returnvalue_4
        (set `local.Local_Hit` _outhit_2)
        (goto _label)))))