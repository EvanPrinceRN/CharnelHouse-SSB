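; BP_CharacterBase is a base character Blueprint that tracks health and death state.
; ChangeHealth adds or subtracts an amount according to its Add flag and clamps the result between zero and HealthMax.
; When health lands on zero it calls TriggerDeath, which only sets the IsDead flag.
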(fn `ChangeHealth`
  (params (Amount :type "Float (double-precision)") (Add :type Boolean))
  (if Add
    (set `self.HealthCurrent` (`KismetMathLibrary.FClamp` (+ (`self.HealthCurrent`) Amount) 0.0 (`self.HealthMax`)))
    (else
      (set `self.HealthCurrent` (`KismetMathLibrary.FClamp` (- (`self.HealthCurrent`) Amount) 0.0 (`self.HealthMax`)))))
  (if (== (`self.HealthCurrent`) 0.0)
    (`self.TriggerDeath`)))

(fn `TriggerDeath`
  (set `self.IsDead` true))

(fn `UserConstructionScript`)