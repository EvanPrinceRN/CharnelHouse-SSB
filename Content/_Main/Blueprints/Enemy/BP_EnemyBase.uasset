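; BP_EnemyBase is a base enemy that takes damage from the player's third-person character and is destroyed when its health runs out.
; AnyDamage ignores other causers and plays a hit montage, using a flag to drop further hits until it finishes.
; On montage completion or interruption, it clears the flag, subtracts a fixed amount of health regardless of incoming damage, and destroys the actor at zero or below.
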(event `self.ReceiveAnyDamage`
  (params (Damage :type "Float (single-precision)") (DamageType :type "DamageType Object Reference") (InstigatedBy :type "Controller Object Reference") (DamageCauser :type "Actor Object Reference"))
  (cast `/Game/_Main/Blueprints/Main_Character/BP_ThirdPersonCharacter` DamageCauser)
  (if (not (`self.Local_HitPlaying`))
    (set `self.Local_HitPlaying` true)
    (`|PlayMontage` (`self.Mesh`) "/Game/_Main/Characters/Enemy1/Animations/Combat/Enemy1OnHit.Enemy1OnHit"
      (:`OnCompleted`
        _)
      (:`OnInterrupted`
        _))
    (set `self.Local_HitPlaying` false)
    (bind _output_get (set `self.Health` (- (`self.Health`) 10.0)))
    (if (<= _output_get 0.0)
      (`self.K2_DestroyActor`))))

(fn `UserConstructionScript`)